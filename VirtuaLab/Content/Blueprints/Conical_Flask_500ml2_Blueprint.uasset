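; Conical 500ml flask Blueprint that shows a timed fire or smoke particle effect.
; Tick polls the IsFire and IsSmoke flags on PlayEffect, with fire taking priority, and activates the matching particle component.
; After a five-second Delay it clears that flag and deactivates the effect.
; BeginPlay, overlap and the construction script are empty.
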(event EventBeginPlay)

(event Collision|EventActorBeginOverlap
  (params (OtherActor :type Actor%20Object%20Reference)))

(event EventTick
  (params (DeltaSeconds :type Float%20%28single-precision%29))
  (if (Variables|/Script/VirtuaLab.PlayEffect|GetisFire (Variables|Default|GetPlayEffect))
    (Components|Activation|Activate (Variables|Default|GetPar_TorchFire_02) false)
    (Utilities|FlowControl|Delay 5.0)
    (Variables|/Script/VirtuaLab.PlayEffect|SetisFire (Variables|Default|GetPlayEffect) false)
    (Components|Activation|Deactivate (Variables|Default|GetPar_TorchFire_02))
    (elif (Variables|/Script/VirtuaLab.PlayEffect|GetisSmoke (Variables|Default|GetPlayEffect))
      (Components|Activation|Activate (Variables|Default|GetP_Smoke) false)
      (Utilities|FlowControl|Delay 5.0)
      (Variables|/Script/VirtuaLab.PlayEffect|SetisSmoke (Variables|Default|GetPlayEffect) false)
      (Components|Activation|Deactivate (Variables|Default|GetP_Smoke)))))

(fn ConstructionScript)